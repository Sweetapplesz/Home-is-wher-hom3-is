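; Pulley actor with a configurable static mesh that shifts while the side-scroller player character is grabbing.
; Each tick during a grab, it line traces 200 units ahead of the character on the Visibility channel.
; Any hit nudges the mesh along its local Y axis by a fixed per-frame step, without checking what was hit or scaling by delta time.
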(event `self.ReceiveTick`
  (params (DeltaSeconds :type "Float (single-precision)"))
  (bind _asside_scroller_character (cast `/Game/SideScrollerBP/Blueprints/SideScrollerCharacter` (`GameplayStatics.GetPlayerCharacter` 0)))
  (if (`/Game/SideScrollerBP/Blueprints/SideScrollerCharacter.Is Grabbing` _asside_scroller_character)
    (bind _returnvalue (`self.K2_GetActorLocation` _asside_scroller_character))
    (bind (_outhit _returnvalue_2) (`KismetSystemLibrary.LineTraceSingle` _returnvalue (+ _returnvalue (* (`self.GetActorForwardVector` _asside_scroller_character) 200.0)) "TraceTypeQuery1"))
    (if _returnvalue_2
      (`SceneComponent.K2_AddLocalOffset` (`self.StaticMesh`) (0.0 5.0 0.0) false false))))

(fn `UserConstructionScript`
  (`StaticMeshComponent.SetStaticMesh` (`self.StaticMesh`) (`self.Mesh`)))