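; Clock Blueprint that spins a clock hand mesh.
; The construction script assigns the Hand mesh to the StaticMesh component.
; Each Tick stores the frame delta in Speed and adds a local pitch rotation of that value times Direction, so the hand turns about one degree per second, scaled by Direction.
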(event `self.ReceiveTick`
  (params (DeltaSeconds :type "Float (single-precision)"))
  (set `self.Speed` DeltaSeconds)
  (`SceneComponent.K2_AddLocalRotation` (`self.StaticMesh`) (`KismetMathLibrary.MakeRotator` 0.0 (* (`self.Speed`) (`self.Direction`))) false false))

(fn `UserConstructionScript`
  (`StaticMeshComponent.SetStaticMesh` (`self.StaticMesh`) (`self.Hand`)))