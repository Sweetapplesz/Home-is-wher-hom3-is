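; A side-scroller platform that rotates in response to the player character jumping.
; Tick polls the character's IsJumpActive flag and calls Move on each tick it is true, as its DoOnce resets immediately.
; Move plays timeline Yep to lerp the mesh's world rotation toward X/Y/Z, with a DoOnce triggering Reverse on update.
; An author note says editor target values need a 20-degree offset below the intended angle.
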(event `self.ReceiveTick`
  (params (DeltaSeconds :type "Float (single-precision)"))
  ;[1 1 1] Checks if character is jumping
  (bind _asside_scroller_character (cast `/Game/SideScrollerBP/Blueprints/SideScrollerCharacter` (`GameplayStatics.GetPlayerCharacter` 0)))
  (if (`/Game/SideScrollerBP/Blueprints/SideScrollerCharacter.IsJumpActive` _asside_scroller_character)
    (`/Engine/EditorBlueprintResources/StandardMacros.DoOnce` false :!label _label
      (:`Completed`
        (`self.Move`)
        (goto _label :!via `Reset`)))))

(event `Move`
  ;[1 1 1] Rotates Platform
  (bind (_direction _newtrack_1) (`Timeline|Yep` :!label _label_2)
    (:`Update`
      (`SceneComponent.K2_SetWorldRotation` (`self.StaticMesh`) (`KismetMathLibrary.RLerp` (struct) (`KismetMathLibrary.MakeRotator` (`self.X`) (`self.Y`) (`self.Z`)) _newtrack_1) false false)
      (`/Engine/EditorBlueprintResources/StandardMacros.DoOnce` false :!label _label_3
        (:`Completed`
          (goto _label_2 :!via `Reverse`))))
    (:`Finished`
      (goto _label_3 :!via `Reset`))))

(fn `UserConstructionScript`)